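; Drifting vegetation effect actor that configures a Niagara particle system when constructed.
; The construction script scales spawn rate by the product of the actor's scale, so emission grows with volume, and passes a vegetation color.
; It reads the global wind angle from the MPC_GlobalEnvironment parameter collection and converts it to a direction vector for the particles.
; The event graph holds no active logic, so wind is sampled only at construction.
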(event EventBeginPlay)

(event Collision|EventActorBeginOverlap
  (params (OtherActor :type Actor%20Object%20Reference)))

(event EventTick
  (params (DeltaSeconds :type Float%20%28single-precision%29)))

(fn ConstructionScript
  (bind _returnvalue (Transformation|GetActorScale3D))
  (bind _niagara (Variables|Default|GetNiagara))
  (Niagara|SetNiagaraVariable(Float) _niagara "SpawnRate" (* (Variables|Default|GetGeneral%20Spawn%20Rate) (* (.x _returnvalue) (.y _returnvalue) (.z _returnvalue))))
  (Effects|Components|ParticleSystem|SetColorParameter _niagara "Color" (Variables|Default|GetVegetation%20Color))
  (bind _returnvalue_2 (Rendering|Material|GetScalarParameterValue "/Game/_Asset/SoStylized/Environment/MPC_GlobalEnvironment.MPC_GlobalEnvironment" "Global Wind Angle" :!class /Script/Engine.KismetMaterialLibrary))
  (bind _output_get (LocalVariables|SetMPC%20Wind%20Direction (* _returnvalue_2 3.6e+02)))
  (Effects|Components|ParticleSystem|SetVectorParameter _niagara "WindDirection" (Math|Vector|MakeVector (* (Math|Trig|Cos(Degrees) _output_get) -1.0) (Math|Trig|Sin(Degrees) _output_get) 0.0)))